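; Hallway glaive trap with front and back swinging blades that kill the first-person player on contact with a leading edge.
; TriggerTrap plays a timeline that rotates two mirrored pivots, fires woosh sounds from child-actor AmbientSounds and updates the swing direction.
; That direction selects which left or right overlap volume on each blade is lethal.
; Blade hits also apply velocity-based impulses to physics-simulating objects.
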(event OnComponentHit(GlaiveFront)
  (params (HitComponent :type Primitive%20Component%20Object%20Reference) (OtherActor :type Actor%20Object%20Reference) (OtherComp :type Primitive%20Component%20Object%20Reference) (NormalImpulse :type Vector :default "0, 0, 0") (Hit :type Hit%20Result%20Structure%20%28by%20ref%29))
  ;[1 1 1] Collision
  (if (Physics|IsSimulatingPhysics OtherComp "None")
    (Physics|AddImpulseatLocation HitComponent (* (Transformation|GetVelocity) 1e+02) (Transformation|GetActorLocation) "None")))

(event OnComponentHit(GlaiveBack)
  (params (HitComponent :type Primitive%20Component%20Object%20Reference) (OtherActor :type Actor%20Object%20Reference) (OtherComp :type Primitive%20Component%20Object%20Reference) (NormalImpulse :type Vector :default "0, 0, 0") (Hit :type Hit%20Result%20Structure%20%28by%20ref%29))
  ;[1 1 1] Collision
  (if (Physics|IsSimulatingPhysics OtherComp "None")
    (Physics|AddImpulseatLocation OtherComp (* (Transformation|GetVelocity) 1e+02) (Transformation|GetActorLocation) "None")))

(event OnComponentBeginOverlap(GlaiveFrontLeft)
  (params (OverlappedComponent :type Primitive%20Component%20Object%20Reference) (OtherActor :type Actor%20Object%20Reference) (OtherComp :type Primitive%20Component%20Object%20Reference) (OtherBodyIndex :type Integer) (bFromSweep :type Boolean) (SweepResult :type Hit%20Result%20Structure%20%28by%20ref%29))
  ;[1 1 1] Kill Player
  (if (not (Variables|Default|GetDirection))
    (if (== (Utilities|GetClass OtherActor) "/Game/Blueprints/FirstPersonCharacter.FirstPersonCharacter_C")
      (bind _asfirst_person_character (Utilities|Casting|CastToFirstPersonCharacter OtherActor))
      (Default|KillPlayer _asfirst_person_character))))

(event OnComponentBeginOverlap(GlaiveFrontRight)
  (params (OverlappedComponent :type Primitive%20Component%20Object%20Reference) (OtherActor :type Actor%20Object%20Reference) (OtherComp :type Primitive%20Component%20Object%20Reference) (OtherBodyIndex :type Integer) (bFromSweep :type Boolean) (SweepResult :type Hit%20Result%20Structure%20%28by%20ref%29))
  ;[1 1 1] Kill Player
  (if (Variables|Default|GetDirection)
    (if (== (Utilities|GetClass OtherActor) "/Game/Blueprints/FirstPersonCharacter.FirstPersonCharacter_C")
      (bind _asfirst_person_character (Utilities|Casting|CastToFirstPersonCharacter OtherActor))
      (Default|KillPlayer _asfirst_person_character))))

(event OnComponentBeginOverlap(GlaiveBackLeft)
  (params (OverlappedComponent :type Primitive%20Component%20Object%20Reference) (OtherActor :type Actor%20Object%20Reference) (OtherComp :type Primitive%20Component%20Object%20Reference) (OtherBodyIndex :type Integer) (bFromSweep :type Boolean) (SweepResult :type Hit%20Result%20Structure%20%28by%20ref%29))
  ;[1 1 1] Kill Player
  (if (Variables|Default|GetDirection)
    (if (== (Utilities|GetClass OtherActor) "/Game/Blueprints/FirstPersonCharacter.FirstPersonCharacter_C")
      (bind _asfirst_person_character (Utilities|Casting|CastToFirstPersonCharacter OtherActor))
      (Default|KillPlayer _asfirst_person_character))))

(event OnComponentBeginOverlap(GlaiveBackRight)
  (params (OverlappedComponent :type Primitive%20Component%20Object%20Reference) (OtherActor :type Actor%20Object%20Reference) (OtherComp :type Primitive%20Component%20Object%20Reference) (OtherBodyIndex :type Integer) (bFromSweep :type Boolean) (SweepResult :type Hit%20Result%20Structure%20%28by%20ref%29))
  ;[1 1 1] Kill Player
  (if (not (Variables|Default|GetDirection))
    (if (== (Utilities|GetClass OtherActor) "/Game/Blueprints/FirstPersonCharacter.FirstPersonCharacter_C")
      (bind _asfirst_person_character (Utilities|Casting|CastToFirstPersonCharacter OtherActor))
      (Default|KillPlayer _asfirst_person_character))))

(event EventTriggerTrap
  (params (Actor :type Actor%20Object%20Reference))
  (bind (_direction _angle _rotdirection) (Timeline|Rotation Play)
    (:Update
      (Variables|Default|SetDirection (Math|Conversions|ToBoolean(Integer) (Math|Float|Truncate _rotdirection)))
      (Transformation|SetRelativeRotation (Variables|Default|GetPivotFront) (Math|Rotator|MakeRotator 0.0 _angle 0.0) false false)
      (Transformation|SetRelativeRotation (Variables|Default|GetPivotBack) (Math|Rotator|MakeRotator 1.8e+02 _angle 1.8e+02) false false))
    (:Woosh
      (Audio|Components|Audio|Play (Variables|Default|GetWooshFront) 0.0))))

(event EventBeginPlay
  (bind _asambient_sound (Utilities|Casting|CastToAmbientSound (Variables|/Script/Engine.ChildActorComponent|GetChildActor (Variables|Default|GetBP_woosh))))
  (Variables|Default|SetWooshFront (Variables|/Script/Engine.AmbientSound|GetAudioComponent _asambient_sound))
  (bind _asambient_sound_2 (Utilities|Casting|CastToAmbientSound (Variables|/Script/Engine.ChildActorComponent|GetChildActor (Variables|Default|GetBP_woosh1))))
  (Variables|Default|SetWooshBack (Variables|/Script/Engine.AmbientSound|GetAudioComponent _asambient_sound_2)))

(fn ConstructionScript
  (|CallParentFunction))