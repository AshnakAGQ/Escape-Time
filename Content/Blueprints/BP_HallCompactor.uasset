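; BP_HallCompactor is a hallway trap with two compactor pieces that move to crush the player.
; TriggerTrap plays stone sounds from two child actors and runs a timeline that moves both pieces along local X, stopping the sounds when it finishes.
; While a piece's kill box is overlapped, its per-update movement delta is added to the player to push them along.
; Overlapping both kill boxes at once kills the player.
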(event OnComponentBeginOverlap(KillBoxL)
  (params (OverlappedComponent :type Primitive%20Component%20Object%20Reference) (OtherActor :type Actor%20Object%20Reference) (OtherComp :type Primitive%20Component%20Object%20Reference) (OtherBodyIndex :type Integer) (bFromSweep :type Boolean) (SweepResult :type Hit%20Result%20Structure%20%28by%20ref%29))
  (Variables|Default|SetOverlapL true)
  (if (Variables|Default|GetOverlapR)
    (bind _asfirst_person_character (Utilities|Casting|CastToFirstPersonCharacter (Game|GetPlayerCharacter 0)))
    (Default|KillPlayer _asfirst_person_character)))

(event OnComponentBeginOverlap(KillBoxR)
  (params (OverlappedComponent :type Primitive%20Component%20Object%20Reference) (OtherActor :type Actor%20Object%20Reference) (OtherComp :type Primitive%20Component%20Object%20Reference) (OtherBodyIndex :type Integer) (bFromSweep :type Boolean) (SweepResult :type Hit%20Result%20Structure%20%28by%20ref%29))
  (Variables|Default|SetOverlapR true)
  (if (Variables|Default|GetOverlapL)
    (bind _asfirst_person_character (Utilities|Casting|CastToFirstPersonCharacter (Game|GetPlayerCharacter 0)))
    (Default|KillPlayer _asfirst_person_character)))

(event OnComponentEndOverlap(KillBoxL)
  (params (OverlappedComponent :type Primitive%20Component%20Object%20Reference) (OtherActor :type Actor%20Object%20Reference) (OtherComp :type Primitive%20Component%20Object%20Reference) (OtherBodyIndex :type Integer))
  (Variables|Default|SetOverlapL false))

(event OnComponentEndOverlap(KillBoxR)
  (params (OverlappedComponent :type Primitive%20Component%20Object%20Reference) (OtherActor :type Actor%20Object%20Reference) (OtherComp :type Primitive%20Component%20Object%20Reference) (OtherBodyIndex :type Integer))
  (Variables|Default|SetOverlapR false))

(event EventTriggerTrap
  (params (Actor :type Actor%20Object%20Reference))
  (bind _returnvalue (Game|GetPlayerCharacter 0))
  (bind _compactorr (Variables|Default|GetCompactorR))
  (bind _compactorl (Variables|Default|GetCompactorL))
  (bind _returnvalue_2 (Transformation|GetWorldLocation _compactorr))
  (bind _returnvalue_3 (Transformation|GetWorldLocation _compactorl))
  (bind _relativelocation (Variables|/Script/Engine.SceneComponent|GetRelativeLocation _compactorr))
  (bind _rootcomponent (Variables|/Script/Engine.Actor|GetRootComponent _returnvalue))
  (bind _relativelocation_2 (Variables|/Script/Engine.SceneComponent|GetRelativeLocation _compactorl))
  (bind _asambient_sound (Utilities|Casting|CastToAmbientSound (Variables|/Script/Engine.ChildActorComponent|GetChildActor (Variables|Default|GetBP_Stone))))
  (bind _asambient_sound_2 (Utilities|Casting|CastToAmbientSound (Variables|/Script/Engine.ChildActorComponent|GetChildActor (Variables|Default|GetBP_Stone1))))
  (Audio|Components|Audio|Play (Variables|/Script/Engine.AmbientSound|GetAudioComponent _asambient_sound) 0.0)
  (bind (_direction _positionr _positionl) (Timeline|Movement Play)
    (:Update
      (Variables|Default|SetLastL _returnvalue_3)
      (Transformation|SetRelativeLocation _compactorl (Math|Vector|MakeVector _positionl (.y _relativelocation_2) (.z _relativelocation_2)) false false)
      (if (Variables|Default|GetOverlapL)
        (Transformation|AddWorldOffset _rootcomponent (- _returnvalue_3 (Variables|Default|GetLastL)) false false))
      (Variables|Default|SetLastR _returnvalue_2)
      (Transformation|SetRelativeLocation _compactorr (Math|Vector|MakeVector _positionr (.y _relativelocation) (.z _relativelocation)) false false)
      (if (Variables|Default|GetOverlapR)
        (Transformation|AddWorldOffset _rootcomponent (- _returnvalue_2 (Variables|Default|GetLastR)) false false)))
    (:Finished
      (Audio|Components|Audio|Stop (Variables|/Script/Engine.AmbientSound|GetAudioComponent _asambient_sound)))))

(fn ConstructionScript
  (|CallParentFunction))