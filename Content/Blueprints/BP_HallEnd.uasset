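; BP_HallEnd is a level-end actor that plays a helicopter takeoff cutscene and signals the end of the game.
; Overlapping TakeoffTrigger cuts the view to this actor, disables player movement and shows the TakeoffPlayer stand-in.
; Timeline_1 moves the stand-in along two axes, then CallEndGame fires.
; After a one-second delay, Timeline_0 animates the Helicopter's relative height.
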(event OnComponentBeginOverlap(TakeoffTrigger)
  (params (OverlappedComponent :type Primitive%20Component%20Object%20Reference) (OtherActor :type Actor%20Object%20Reference) (OtherComp :type Primitive%20Component%20Object%20Reference) (OtherBodyIndex :type Integer) (bFromSweep :type Boolean) (SweepResult :type Hit%20Result%20Structure%20%28by%20ref%29))
  (bind _takeoffplayer (Variables|Default|GetTakeoffPlayer))
  (bind _helicopter (Variables|Default|GetHelicopter))
  (bind _relativelocation (Variables|/Script/Engine.SceneComponent|GetRelativeLocation _helicopter))
  (Game|Player|SetViewTargetwithBlend (Game|GetPlayerController 0) self 0.0 "VTBlend_Linear" 0.0 false)
  (Pawn|Components|CharacterMovement|SetMovementMode (Variables|/Script/Engine.Character|GetCharacterMovement (Game|GetPlayerCharacter 0)) "MOVE_None" 0)
  (Rendering|SetVisibility (Variables|Default|GetTakeoffPlayer) true false)
  (bind (_direction _positiony _positionz) (Timeline|Timeline_1 Play)
    (:Update
      (Transformation|SetRelativeLocation _takeoffplayer (Math|Vector|MakeVector _positiony 0.0 _positionz) false false))
    (:Finished
      (Rendering|SetVisibility _takeoffplayer true false)
      (Default|CallEndGame)
      (Utilities|FlowControl|Delay 1.0)
      (bind _position (Timeline|Timeline_0 Play)
        (:Update
          (Transformation|SetRelativeLocation _helicopter (Math|Vector|MakeVector (.x _relativelocation) (.y _relativelocation) _position) false false))))))

(event EventBeginPlay)

(event Collision|EventActorBeginOverlap
  (params (OtherActor :type Actor%20Object%20Reference)))

(event EventTick
  (params (DeltaSeconds :type Float%20%28single-precision%29)))

(fn ConstructionScript
  (|CallParentFunction))