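; BP_HallStart is an interactive pedestal that gives the player the pocket watch and sets off a trap.
; Overlap events on Collision track proximity, gating the Activate input.
; On activation it calls GetClock on the FirstPersonCharacter, destroys the watch, collision and barrier, then calls TriggerTrap.
; The PedistalMovement timeline then drives the pedestal's relative height.
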(event OnComponentBeginOverlap(Collision)
  (params (OverlappedComponent :type Primitive%20Component%20Object%20Reference) (OtherActor :type Actor%20Object%20Reference) (OtherComp :type Primitive%20Component%20Object%20Reference) (OtherBodyIndex :type Integer) (bFromSweep :type Boolean) (SweepResult :type Hit%20Result%20Structure%20%28by%20ref%29))
  (Variables|Default|SetCharacter%20Near? true))

(event OnComponentEndOverlap(Collision)
  (params (OverlappedComponent :type Primitive%20Component%20Object%20Reference) (OtherActor :type Actor%20Object%20Reference) (OtherComp :type Primitive%20Component%20Object%20Reference) (OtherBodyIndex :type Integer))
  (Variables|Default|SetCharacter%20Near? false))

(event Input|ActionEvents|InputActionActivate
  (params (Key :type Key%20Structure))
  (bind _pedestal (Variables|Default|GetPedestal))
  (bind _relativelocation (Variables|/Script/Engine.SceneComponent|GetRelativeLocation _pedestal))
  (:Pressed
    (if (Variables|Default|GetCharacter%20Near?)
      (bind _asfirst_person_character (Utilities|Casting|CastToFirstPersonCharacter (Game|GetPlayerCharacter 0)))
      (Default|GetClock _asfirst_person_character)
      (Components|DestroyComponent (Variables|Default|GetBP_PocketWatch))
      (CallFunction|TriggerTrap)
      (bind _movement (Timeline|Pedistal%20Movement Play)
        (:Update
          (Transformation|SetRelativeLocation _pedestal (Math|Vector|MakeVector (.x _relativelocation) (.y _relativelocation) _movement) false false))))))

(fn ConstructionScript
  (|CallParentFunction))