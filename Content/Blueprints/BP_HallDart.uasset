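; Hallway dart trap that fires BP_Dart actors from a left and a right spawn point when TriggerTrap is called.
; A timeline named Tick drives the firing, with separate event tracks spawning darts at DartSpawnL and DartSpawnR.
; Each dart takes its spawn point's rotation and a random world Y and Z offset to scatter the volley.
; Each spawned dart also gets a child actor component added.
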(event EventTriggerTrap
  (params (Actor :type Actor%20Object%20Reference))
  (bind _dartspawnr (Variables|Default|GetDartSpawnR))
  (bind _dartspawnl (Variables|Default|GetDartSpawnL))
  (bind _returnvalue (Transformation|GetWorldLocation _dartspawnr))
  (bind _returnvalue_2 (Transformation|GetWorldLocation _dartspawnl))
  (Timeline|Tick Play
    (:Spawn
      (bind _returnvalue_3 (Game|SpawnActorfromClass "/Game/Blueprints/BP_Dart.BP_Dart_C" (Math|Transform|MakeTransform (Math|Vector|MakeVector (.x _returnvalue_2) (+ (.y _returnvalue_2) (Math|Random|RandomFloatinRange -3e+02 3e+02)) (+ (.z _returnvalue_2) (Math|Random|RandomFloatinRange -2e+02 2e+02))) (Transformation|GetWorldRotation _dartspawnl)) "Undefined" 0 0))
      (AddComponent|AddChildActorComponent _returnvalue_3 false))
    (:SpawnB
      (bind _returnvalue_4 (Game|SpawnActorfromClass "/Game/Blueprints/BP_Dart.BP_Dart_C" (Math|Transform|MakeTransform (Math|Vector|MakeVector (.x _returnvalue) (+ (.y _returnvalue) (Math|Random|RandomFloatinRange -3e+02 3e+02)) (+ (.z _returnvalue) (Math|Random|RandomFloatinRange -2e+02 2e+02))) (Transformation|GetWorldRotation _dartspawnr)) "Undefined" 0 0))
      (AddComponent|AddChildActorComponent _returnvalue_4 false))))

(fn ConstructionScript
  (|CallParentFunction))