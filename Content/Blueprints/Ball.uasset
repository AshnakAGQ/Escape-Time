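; A rolling boulder hazard that kills the first-person player when its box or sphere collision overlaps them.
; On BeginPlay it takes hit and roll audio components from child AmbientSound actors.
; Ground collision overlaps play the impact and start the rolling sound, which stops on end overlap once at most one overlapping actor remains.
; An unconnected timeline would scale roll volume by horizontal physics speed but never runs.
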(event OnComponentBeginOverlap(BoxCollision)
  (params (OverlappedComponent :type Primitive%20Component%20Object%20Reference) (OtherActor :type Actor%20Object%20Reference) (OtherComp :type Primitive%20Component%20Object%20Reference) (OtherBodyIndex :type Integer) (bFromSweep :type Boolean) (SweepResult :type Hit%20Result%20Structure%20%28by%20ref%29))
  ;[1 1 1] Ball: Crush Logic
  (bind _asfirst_person_character (Utilities|Casting|CastToFirstPersonCharacter OtherActor))
  (Default|KillPlayer _asfirst_person_character))

(event OnComponentBeginOverlap(SphereCollision)
  (params (OverlappedComponent :type Primitive%20Component%20Object%20Reference) (OtherActor :type Actor%20Object%20Reference) (OtherComp :type Primitive%20Component%20Object%20Reference) (OtherBodyIndex :type Integer) (bFromSweep :type Boolean) (SweepResult :type Hit%20Result%20Structure%20%28by%20ref%29))
  ;[1 1 1] Ball: Crush Logic
  (bind _asfirst_person_character (Utilities|Casting|CastToFirstPersonCharacter OtherActor))
  (Default|KillPlayer _asfirst_person_character))

(event OnComponentBeginOverlap(GroundCollision)
  (params (OverlappedComponent :type Primitive%20Component%20Object%20Reference) (OtherActor :type Actor%20Object%20Reference) (OtherComp :type Primitive%20Component%20Object%20Reference) (OtherBodyIndex :type Integer) (bFromSweep :type Boolean) (SweepResult :type Hit%20Result%20Structure%20%28by%20ref%29))
  (CallFunction|PlaySoundLand OtherActor)
  (CallFunction|PlaySoundRolling OtherActor))

(event OnComponentEndOverlap(GroundCollision)
  (params (OverlappedComponent :type Primitive%20Component%20Object%20Reference) (OtherActor :type Actor%20Object%20Reference) (OtherComp :type Primitive%20Component%20Object%20Reference) (OtherBodyIndex :type Integer))
  (CallFunction|StopSoundRolling OtherActor))

(event Custom|PlaySoundRolling
  (params (Other%20Actor :type Actor%20Object%20Reference))
  (bind _roll (Variables|Default|GetRoll))
  (if (not (Audio|Components|Audio|IsPlaying _roll))
    (Audio|Components|Audio|Play _roll 0.0)))

(event Custom|StopSoundRolling
  (params (Other%20Actor :type Actor%20Object%20Reference))
  (bind _roll (Variables|Default|GetRoll))
  (if (<= (Utilities|Array|Length (Collision|GetOverlappingActors (Variables|Default|GetGroundCollision) 0 :!class /Script/Engine.PrimitiveComponent)) 1)
    (if (Audio|Components|Audio|IsPlaying _roll)
      (Audio|Components|Audio|Stop _roll))))

(event Custom|PlaySoundLand
  (params (Other%20Actor :type Actor%20Object%20Reference))
  (Audio|Components|Audio|Play (Variables|Default|GetHit) 0.0))

(event EventBeginPlay
  (bind _asambient_sound (Utilities|Casting|CastToAmbientSound (Variables|/Script/Engine.ChildActorComponent|GetChildActor (Variables|Default|GetSoundHit))))
  (bind _output_get (Variables|Default|SetHit (Variables|/Script/Engine.AmbientSound|GetAudioComponent _asambient_sound)))
  (Audio|Components|Audio|SetVolumeMultiplier _output_get 0.0 :!class /Script/Engine.AudioComponent)
  (Components|Activation|Activate _output_get false)
  (Audio|Components|Audio|SetVolumeMultiplier _output_get 1.0 :!class /Script/Engine.AudioComponent)
  (bind _asambient_sound_2 (Utilities|Casting|CastToAmbientSound (Variables|/Script/Engine.ChildActorComponent|GetChildActor (Variables|Default|GetSoundRoll))))
  (bind _output_get_2 (Variables|Default|SetRoll (Variables|/Script/Engine.AmbientSound|GetAudioComponent _asambient_sound_2)))
  (Audio|Components|Audio|SetVolumeMultiplier _output_get_2 0.0 :!class /Script/Engine.AudioComponent)
  (Components|Activation|Activate _output_get_2 false)
  (Audio|Components|Audio|SetVolumeMultiplier _output_get_2 1.0 :!class /Script/Engine.AudioComponent))

(fn ConstructionScript)