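; BP_HallHole is a trapdoor pit trap with acid that kills the first-person player.
; TriggerTrap plays two child-actor ambient sounds while a timeline pitches the left and right door pivots.
; When the timeline finishes, the sounds stop and both trapdoors lose collision.
; Overlapping the acid calls KillPlayer on the character, then attaches a child actor and particle system to it.
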(event OnComponentBeginOverlap(Acid)
  (params (OverlappedComponent :type Primitive%20Component%20Object%20Reference) (OtherActor :type Actor%20Object%20Reference) (OtherComp :type Primitive%20Component%20Object%20Reference) (OtherBodyIndex :type Integer) (bFromSweep :type Boolean) (SweepResult :type Hit%20Result%20Structure%20%28by%20ref%29))
  (bind _asfirst_person_character (Utilities|Casting|CastToFirstPersonCharacter OtherActor))
  (Default|KillPlayer _asfirst_person_character)
  (AddComponent|AddChildActorComponent OtherActor false)
  (AddComponent|AddParticleSystemComponent OtherActor false))

(event EventTriggerTrap
  (params (Actor :type Actor%20Object%20Reference))
  (bind _lpivot (Variables|Default|GetLPivot))
  (bind _rpivot (Variables|Default|GetRPivot))
  (bind _relativerotation (Variables|/Script/Engine.SceneComponent|GetRelativeRotation _rpivot))
  (bind _relativerotation_2 (Variables|/Script/Engine.SceneComponent|GetRelativeRotation _lpivot))
  (bind _asambient_sound (Utilities|Casting|CastToAmbientSound (Variables|/Script/Engine.ChildActorComponent|GetChildActor (Variables|Default|GetBP_Stone))))
  (bind _asambient_sound_2 (Utilities|Casting|CastToAmbientSound (Variables|/Script/Engine.ChildActorComponent|GetChildActor (Variables|Default|GetBP_Stone2))))
  (Audio|Components|Audio|Play (Variables|/Script/Engine.AmbientSound|GetAudioComponent _asambient_sound) 0.0)
  (bind _rotation (Timeline|Rotation Play)
    (:Update
      (Transformation|SetRelativeRotation _lpivot (Math|Rotator|MakeRotator (.roll _relativerotation_2) _rotation (.yaw _relativerotation_2)) false false)
      (Transformation|SetRelativeRotation _rpivot (Math|Rotator|MakeRotator (.roll _relativerotation) _rotation (.yaw _relativerotation)) false false))
    (:Finished
      (Audio|Components|Audio|Stop (Variables|/Script/Engine.AmbientSound|GetAudioComponent _asambient_sound))
      (Collision|SetCollisionEnabled (Variables|Default|GetTrapdoorL) "NoCollision")
      (Collision|SetCollisionEnabled (Variables|Default|GetTrapdoorR) "NoCollision"))))

(fn ConstructionScript
  (|CallParentFunction))