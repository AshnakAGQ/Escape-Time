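; BP_HallBall is a crushing trap that kills the player caught between its top and bottom kill boxes.
; TriggerTrap plays a timeline that drives the relative Z of HallBallTop, with a child-actor ambient sound playing until the motion finishes.
; Each kill box tracks an overlap flag without filtering the overlapping actor, and when both are set it calls KillPlayer on the FirstPersonCharacter.
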(event OnComponentBeginOverlap(KillBoxTop)
  (params (OverlappedComponent :type Primitive%20Component%20Object%20Reference) (OtherActor :type Actor%20Object%20Reference) (OtherComp :type Primitive%20Component%20Object%20Reference) (OtherBodyIndex :type Integer) (bFromSweep :type Boolean) (SweepResult :type Hit%20Result%20Structure%20%28by%20ref%29))
  ;[1 1 1] Crush Logic
  (Variables|Default|SetOverlapTop true)
  (if (Variables|Default|GetOverlapBottom)
    (bind _asfirst_person_character (Utilities|Casting|CastToFirstPersonCharacter (Game|GetPlayerCharacter 0)))
    (Default|KillPlayer _asfirst_person_character)))

(event OnComponentBeginOverlap(KillBoxBottom)
  (params (OverlappedComponent :type Primitive%20Component%20Object%20Reference) (OtherActor :type Actor%20Object%20Reference) (OtherComp :type Primitive%20Component%20Object%20Reference) (OtherBodyIndex :type Integer) (bFromSweep :type Boolean) (SweepResult :type Hit%20Result%20Structure%20%28by%20ref%29))
  ;[1 1 1] Crush Logic
  (Variables|Default|SetOverlapBottom true)
  (if (Variables|Default|GetOverlapTop)
    (bind _asfirst_person_character (Utilities|Casting|CastToFirstPersonCharacter (Game|GetPlayerCharacter 0)))
    (Default|KillPlayer _asfirst_person_character)))

(event OnComponentEndOverlap(KillBoxTop)
  (params (OverlappedComponent :type Primitive%20Component%20Object%20Reference) (OtherActor :type Actor%20Object%20Reference) (OtherComp :type Primitive%20Component%20Object%20Reference) (OtherBodyIndex :type Integer))
  ;[1 1 1] Crush Logic
  (Variables|Default|SetOverlapTop false))

(event OnComponentEndOverlap(KillBoxBottom)
  (params (OverlappedComponent :type Primitive%20Component%20Object%20Reference) (OtherActor :type Actor%20Object%20Reference) (OtherComp :type Primitive%20Component%20Object%20Reference) (OtherBodyIndex :type Integer))
  ;[1 1 1] Crush Logic
  (Variables|Default|SetOverlapBottom false))

(event EventTriggerTrap
  (params (Actor :type Actor%20Object%20Reference))
  (bind _hallballtop (Variables|Components|GetHallBallTop))
  (bind _relativelocation (Variables|/Script/Engine.SceneComponent|GetRelativeLocation _hallballtop))
  ;[1 1 1] Trap Trigger
  (bind _asambient_sound (Utilities|Casting|CastToAmbientSound (Variables|/Script/Engine.ChildActorComponent|GetChildActor (Variables|Default|GetBP_Stone))))
  (Audio|Components|Audio|Play (Variables|/Script/Engine.AmbientSound|GetAudioComponent _asambient_sound) 0.0)
  (bind _movement (Timeline|Top Play)
    (:Update
      (Transformation|SetRelativeLocation _hallballtop (Math|Vector|MakeVector (.x _relativelocation) (.y _relativelocation) _movement) false false))
    (:Finished
      (Audio|Components|Audio|Stop (Variables|/Script/Engine.AmbientSound|GetAudioComponent _asambient_sound)))))

(fn ConstructionScript
  (|CallParentFunction))