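; BP_Dart is a projectile that kills the first-person player character on contact.
; Its Hit event pushes any physics-simulating component with an impulse scaled from the dart's velocity, and calls KillPlayer when the hit actor's class is FirstPersonCharacter.
; Any hit also starts a short delay, after which the dart destroys itself.
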(event Collision|EventHit
  (params (MyComp :type Primitive%20Component%20Object%20Reference) (Other :type Actor%20Object%20Reference) (OtherComp :type Primitive%20Component%20Object%20Reference) (bSelfMoved :type Boolean) (HitLocation :type Vector :default "0, 0, 0") (HitNormal :type Vector :default "0, 0, 0") (NormalImpulse :type Vector :default "0, 0, 0") (Hit :type Hit%20Result%20Structure%20%28by%20ref%29))
  ;[1 1 1] Collision
  (Utilities|FlowControl|Sequence
    (:then_0
      (if (Physics|IsSimulatingPhysics OtherComp "None")
        (Physics|AddImpulseatLocation OtherComp (* (Transformation|GetVelocity) 1e+02) (Transformation|GetActorLocation) "None")))
    (:then_1
      (if (== (Utilities|GetClass Other) "/Game/Blueprints/FirstPersonCharacter.FirstPersonCharacter_C")
        (bind _asfirst_person_character (Utilities|Casting|CastToFirstPersonCharacter Other))
        (Default|KillPlayer _asfirst_person_character)))
    (:then_2
      (Utilities|FlowControl|Delay 2.0)
      (Actor|DestroyActor))))

(fn ConstructionScript)